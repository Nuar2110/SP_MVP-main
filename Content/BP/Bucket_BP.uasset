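; Bucket Blueprint for a fire-fighting task, holding a fire effect and sound that are put out through damage.
; MakeDamage lowers HitPoints and rescales the fire from its BeginPlay scale, shrinking it linearly from full to half size as health goes from 100 to zero.
; At zero or below, it deactivates the fire, stops the sound, detaches the FireExtinguisher and tells TaskManager to change task.
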(event Custom|MakeDamage
  (params (DamageTaken :type Float%20%28single-precision%29))
  (Variables|Default|SetHitPoints (- (Variables|Default|GetHitPoints) DamageTaken))
  (CallFunction|ChangeFireScale)
  (CallFunction|CheckIsDefeated))

(event Custom|CheckIsDefeated
  (if (<= (Variables|Default|GetHitPoints) 0.0)
    (Components|Activation|Deactivate (Variables|Default|GetFire_04))
    (Audio|Components|Audio|Stop (Variables|Default|GetFireSound))
    (Default|DetachfromActor (Variables|Default|GetFireExtinguisher))
    (Default|ChangeTask (Variables|Default|GetTaskManager))))

(event Custom|ChangeFireScale
  (Transformation|SetWorldScale3D (Variables|Default|GetFire_04) (* (Variables|Default|GetFireScaleDefault) (/ (+ (/ (- 1e+02 (Variables|Default|GetHitPoints)) 2.0) (Variables|Default|GetHitPoints)) 1e+02))))

(event EventBeginPlay
  (Variables|Default|SetFireScaleDefault (Transformation|GetWorldScale (Variables|Default|GetFire_04))))

(event Collision|EventActorBeginOverlap
  (params (OtherActor :type Actor%20Object%20Reference)))

(event EventTick
  (params (DeltaSeconds :type Float%20%28single-precision%29)))

(fn ConstructionScript)